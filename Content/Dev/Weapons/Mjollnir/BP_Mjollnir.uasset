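; Mjollnir, a VR throwable hammer that registers itself as the grabbing hand's remote-grab component on the VRPawn.
; Dropping sets a flight direction from averaged hand-grab velocity, and grabbing clears it.
; While free, Tick moves it in a straight swept line at FlySpeed, facing its heading.
; Swept hits ragdoll Characters and apply mass-scaled force to them or to simulating physics components.
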(event `self.GrabComponent.OnGrabbed`
  (params (SelfRef :type "/Game/VRTemplate/Blueprints/GrabComponent Object Reference"))
  (set `self.Direction` (0.0 0.0 0.0))
  (bind _asvrpawn (cast `/Game/VRTemplate/Blueprints/VRPawn` (`ActorComponent.GetOwner` (`/Game/VRTemplate/Blueprints/GrabComponent.MotionControllerRef` SelfRef))))
  (if (`|EnumEquality` (`/Game/VRTemplate/Blueprints/GrabComponent.GetHeldByHand` SelfRef) "Left")
    (set `/Game/VRTemplate/Blueprints/VRPawn.RemoteGrabComponentLeft` SelfRef _asvrpawn)
    (else
      (set `/Game/VRTemplate/Blueprints/VRPawn.RemoteGrabComponentRight` SelfRef _asvrpawn))))

(event `self.GrabComponent.OnDropped`
  (params (SeflRef :type "/Game/VRTemplate/Blueprints/GrabComponent Object Reference"))
  (set `self.Direction` (`KismetMathLibrary.Normal` (`/Game/VRTemplate/Blueprints/GrabComponent.GetAverageVector` SeflRef (`/Game/VRTemplate/Blueprints/GrabComponent.LinearVelocity` SeflRef)))))

(event `self.ReceiveTick`
  (params (DeltaSeconds :type "Float (single-precision)"))
  (bind _grabcomponent (`self.GrabComponent`))
  (if (and (not (`/Game/VRTemplate/Blueprints/GrabComponent.bIsHeld` _grabcomponent)) (not (`/Game/VRTemplate/Blueprints/GrabComponent.bIsPulled` _grabcomponent)) (not (`KismetSystemLibrary.IsValid` (`SceneComponent.GetAttachParent` (`self.WeaponMesh`)))) (not (`KismetMathLibrary.Vector_IsZero` (`self.Direction`))))
    (`self.K2_SetActorRotation` (`KismetMathLibrary.Conv_VectorToRotator` (`self.Direction`)) true)
    (bind _sweephitresult (`self.K2_SetActorLocation` (+ (`self.K2_GetActorLocation`) (* (`self.Direction`) (`self.FlySpeed`) DeltaSeconds)) true))
    (bind (_bblockinghit _binitialoverlap _time _distance _location _impactpoint _normal _impactnormal _physmat _hitactor _hitcomponent) (`GameplayStatics.BreakHitResult` _sweephitresult))
    (`/Engine/EditorBlueprintResources/StandardMacros.IsValid` _hitcomponent
      (:`Is Valid`
        (bind _ascharacter (cast `Character` _hitactor)
          (:`then`
            (`PrimitiveComponent.SetCollisionEnabled` (`Character.CapsuleComponent` _ascharacter) "NoCollision")
            (bind _mesh (`Character.Mesh` _ascharacter))
            (`/Engine/EditorBlueprintResources/StandardMacros.IsValid` _mesh
              (:`Is Valid`
                (`PrimitiveComponent.SetCollisionProfileName` _mesh "Ragdoll" true)
                (`PrimitiveComponent.SetSimulatePhysics` _mesh true)
                (`PrimitiveComponent.WakeAllRigidBodies` _mesh)
                (`PrimitiveComponent.AddForce` _mesh (* (`self.Direction`) (`self.FlySpeed`) (`self.Force`) (`PrimitiveComponent.GetMass` _mesh)) "None" true))))
          (:`CastFailed`
            (if (`SceneComponent.IsSimulatingPhysics` _hitcomponent "None")
              (`PrimitiveComponent.AddForce` _hitcomponent (* (`self.Direction`) (`self.FlySpeed`) (`self.Force`) (`PrimitiveComponent.GetMass` _hitcomponent)) "None" true))))))))

(fn `UserConstructionScript`)